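; Shed trigger Blueprint, likely for opening and closing the shed, that drives a Level Sequence from a Sphere overlap.
; Begin overlap plays the sequence forward and end overlap plays it in reverse, with no filter on the overlapping actor.
; Two DoOnce nodes reset each other to alternate the directions, and each playback creates a new sequence player.
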(event `self.Sphere.OnComponentBeginOverlap`
  (params (OverlappedComponent :type "PrimitiveComponent Object Reference") (OtherActor :type "Actor Object Reference") (OtherComp :type "PrimitiveComponent Object Reference") (OtherBodyIndex :type Integer) (bFromSweep :type Boolean) (SweepResult :type "HitResult Structure (by ref)"))
  (`/Engine/EditorBlueprintResources/StandardMacros.DoOnce` false :!label _label
    (:`Completed`
      (bind _outactor (`LevelSequencePlayer.CreateLevelSequencePlayer` (`self.LevelSequence`)))
      (`MovieSceneSequencePlayer.Play` (`LevelSequenceActor.SequencePlayer` _outactor))
      (goto _label_2 :!via `Reset`))))

(event `self.Sphere.OnComponentEndOverlap`
  (params (OverlappedComponent :type "PrimitiveComponent Object Reference") (OtherActor :type "Actor Object Reference") (OtherComp :type "PrimitiveComponent Object Reference") (OtherBodyIndex :type Integer))
  (`/Engine/EditorBlueprintResources/StandardMacros.DoOnce` true :!label _label_2
    (:`Completed`
      (bind _outactor (`LevelSequencePlayer.CreateLevelSequencePlayer` (`self.LevelSequence`)))
      (`MovieSceneSequencePlayer.PlayReverse` (`LevelSequenceActor.SequencePlayer` _outactor))
      (goto _label :!via `Reset`))))

(fn `UserConstructionScript`)